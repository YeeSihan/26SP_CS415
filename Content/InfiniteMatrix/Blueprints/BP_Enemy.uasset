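; BP_Enemy is an enemy actor that reacts to sphere overlaps with the player or a projectile.
; On overlap with BP_Player, it calls the player's ProcessHit and destroys itself.
; On overlap with BP_Projectile, it runs GameOver, which despite its name only adds DestroyScore to the player pawn's score and destroys the enemy.
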(event OnComponentBeginOverlap(Sphere)
  (params (OverlappedComponent :type Primitive%20Component%20Object%20Reference) (OtherActor :type Actor%20Object%20Reference) (OtherComp :type Primitive%20Component%20Object%20Reference) (OtherBodyIndex :type Integer) (bFromSweep :type Boolean) (SweepResult :type Hit%20Result%20Structure%20%28by%20ref%29))
  (Utilities|FlowControl|Sequence
    (:then_0
      (bind _asbp_player (Utilities|Casting|CastToBP_Player OtherActor))
      (Default|ProcessHit _asbp_player)
      (Actor|DestroyActor))
    (:then_1
      (Utilities|Casting|CastToBP_Projectile OtherActor)
      (CallFunction|GameOver))))

(event EventBeginPlay)

(event Collision|EventActorBeginOverlap
  (params (OtherActor :type Actor%20Object%20Reference)))

(event EventTick
  (params (DeltaSeconds :type Float%20%28single-precision%29)))

(fn ConstructionScript)

(fn GameOver
  (bind _asbp_player (Utilities|Casting|CastToBP_Player (Game|Player|GetPlayerPawn 0)))
  (Default|AddScore _asbp_player (Variables|Default|GetDestroy_score))
  (Actor|DestroyActor))